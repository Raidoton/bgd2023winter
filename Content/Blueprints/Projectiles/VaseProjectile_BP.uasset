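; Vase projectile that bounces off a pillow, then adds or removes a player point depending on whether it hits a cloud or a rock.
; The first PillowHit sets the projectile movement velocity straight up and sets a flag that blocks further bounces.
; CloudHit and RockHit act only after that bounce, calling AddPoints on player character 0 to award or deduct the point, then destroying the vase.
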(event `self.PillowHit`
  (if (not (`self.HasHitPillow?`))
    (set `MovementComponent.Velocity` (0.0 0.0 400.0) (`self.ProjectileMovement`))
    (set `self.HasHitPillow?` true)))

(event `self.CloudHit`
  (if (`self.HasHitPillow?`)
    (bind _asplayer_character_bp (cast `/Game/Blueprints/PlayerCharacter_BP` (`GameplayStatics.GetPlayerCharacter` 0)))
    (`/Game/Blueprints/PlayerCharacter_BP.AddPoints` _asplayer_character_bp 1)
    (`self.K2_DestroyActor`)))

(event `self.RockHit`
  (if (`self.HasHitPillow?`)
    (bind _asplayer_character_bp (cast `/Game/Blueprints/PlayerCharacter_BP` (`GameplayStatics.GetPlayerCharacter` 0)))
    (`/Game/Blueprints/PlayerCharacter_BP.AddPoints` _asplayer_character_bp -1)
    (`self.K2_DestroyActor`)))

(fn `UserConstructionScript`
  (`parent.UserConstructionScript`))