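; Base projectile Blueprint that reacts to the type of surface it overlaps.
; On StaticMesh overlap, it reads the physical material of the other component's first material and switches on surface type to Player, Pillow, Rock or Cloud hit events.
; These events are empty here, apparently left for child Blueprints to override.
; The construction script copies the initial speed and gravity scale variables into ProjectileMovement.
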(event `self.StaticMesh.OnComponentBeginOverlap`
  (params (OverlappedComponent :type "PrimitiveComponent Object Reference") (OtherActor :type "Actor Object Reference") (OtherComp :type "PrimitiveComponent Object Reference") (OtherBodyIndex :type Integer) (bFromSweep :type Boolean) (SweepResult :type "HitResult Structure (by ref)"))
  (bind _returnvalue (`PrimitiveComponent.GetMaterial` OtherComp 0))
  ;[1 1 1] On Overlap
  (`/Engine/EditorBlueprintResources/StandardMacros.IsValid` _returnvalue
    (:`Is Valid`
      (switch `EPhysicalSurface` (`PhysicalMaterial.SurfaceType` (`MaterialInterface.GetPhysicalMaterial` _returnvalue))
        (:`SurfaceType1`
          (`self.PlayerHit`))
        (:`SurfaceType2`
          (`self.PillowHit`))
        (:`SurfaceType3`
          (`self.RockHit`))
        (:`SurfaceType4`
          (`self.CloudHit`))))))

(event `PillowHit`
  ;[1 1 1] Hit Events
)

(event `CloudHit`
  ;[1 1 1] Hit Events
)

(event `RockHit`
  ;[1 1 1] Hit Events
)

(event `PlayerHit`
  ;[1 1 1] Hit Events
)

(fn `UserConstructionScript`
  (bind _projectilemovement (`self.ProjectileMovement`))
  (set `ProjectileMovementComponent.InitialSpeed` (`self.InitialSpeed`) _projectilemovement)
  (set `ProjectileMovementComponent.ProjectileGravityScale` (`self.GravityScale`) _projectilemovement))